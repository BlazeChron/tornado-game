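; Tornado actor that swirls, pulls in and lifts characters and physics objects inside its capsule.
; Each tick it applies CalculateTornadoForce to overlapping components, through CharacterMovement for characters and directly for simulating bodies.
; The force sums a mass-scaled horizontal pull to center, steering toward a tangential velocity from a cross product, and gravity-relative lift set by UpwardThrustMultiplier.
; An InnerRadius distance check is left unused.
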(event EventBeginPlay)

(event Collision|EventActorBeginOverlap
  (params (OtherActor :type Actor%20Object%20Reference)))

(event EventTick
  (params (DeltaSeconds :type Float%20%28single-precision%29))
  (bind _capsule (Variables|Default|GetCapsule))
  (bind _outoverlappingcomponents (Class|PrimitiveComponent|GetOverlappingComponents _capsule))
  (if (!= (Utilities|Array|Length _outoverlappingcomponents) 0)
    (for _array_element _outoverlappingcomponents
      (bind _ascharacter (Utilities|Casting|CastToCharacter (Components|GetOwner _array_element))
        (:then
          (bind _resultforce (CallFunction|CalculateTornadoForce (Transformation|GetWorldLocation (Variables|/Script/Engine.MovementComponent|GetUpdatedPrimitive (Variables|/Script/Engine.Character|GetCharacterMovement _ascharacter))) (Pawn|Components|CharacterMovement|GetLastUpdateVelocity (Variables|/Script/Engine.Character|GetCharacterMovement _ascharacter)) (Variables|/Script/Engine.CharacterMovementComponent|GetMass (Variables|/Script/Engine.Character|GetCharacterMovement _ascharacter))))
          (Physics|AddForce (Variables|/Script/Engine.Character|GetCharacterMovement _ascharacter) _resultforce))
        (:CastFailed
          (if (Physics|IsSimulatingPhysics _array_element "None")
            (bind _resultforce_2 (CallFunction|CalculateTornadoForce (Transformation|GetWorldLocation _array_element) (Transformation|GetComponentVelocity _array_element) (Physics|GetMass _array_element)))
            (Physics|AddForce _array_element _resultforce_2 "None" false)))))))

(fn ConstructionScript)

(fn CalculateTornadoForce
  (params (ObjectLocation :type Vector) (ObjectVelocity :type Vector) (ObjectMass :type Float%20%28double-precision%29))
  (bind _returnvalue (Transformation|GetActorLocation))
  (bind _returnvalue_2 (- _returnvalue ObjectLocation))
  (bind _returnvalue_3 (Math|Vector|MakeVector (.x _returnvalue_2) (.y _returnvalue_2) 0.0))
  (return (+ (* _returnvalue_3 ObjectMass) (+ (* (- (Math|Vector|CrossProduct _returnvalue_3 "0.000000,0.000000,1.000000") ObjectVelocity) 1e+03) (Math|Vector|MakeVector 0.0 0.0 (* (* (Variables|Default|GetUpwardThrustMultiplier) 981.0) ObjectMass))))))