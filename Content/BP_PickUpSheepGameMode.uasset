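; Game mode for a sheep pick-up level that declares a win when the fence's enter event fires.
; On BeginPlay it finds the first BP_Fence in the level and binds YouWin to that fence's OnEnter event, printing an error if none exists.
; The win is only a printed message, and Tick is unused.
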(event Custom|YouWin
  (Development|PrintString "You win"))

(event EventBeginPlay
  (Development|PrintString "PickUpSheepMode")
  (bind _outactors (Actor|GetAllActorsOfClass "/Game/BP_Fence.BP_Fence_C"))
  (if (> (Utilities|Array|Length _outactors) 0)
    (Variables|Default|SetFence (Utilities|Array|Get(acopy) _outactors))
    (EventDispatchers|BindEventtoOnEnter (Variables|Default|GetFence) (delegate Custom|YouWin))
    (else
      (Development|PrintString "Error! No fence"))))

(event EventTick
  (params (DeltaSeconds :type Float%20%28single-precision%29)))

(fn ConstructionScript)